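; BP_SinglePlayer_GameMode is the single-player game mode that starts play by spawning a shape at the level's block spawner.
; On BeginPlay it caches the first BP_BlockSpawner's transform, calls SpawnShape and binds an event to game over.
; SpawnShape spawns a random class from Shapes, though its Length - 1 bound never selects the last entry.
; OnGameOver and Tick are empty.
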(event `self.ReceiveBeginPlay`
  (bind _outactors (`GameplayStatics.GetAllActorsOfClass` "/Game/Blueprints/BP_BlockSpawner.BP_BlockSpawner_C"))
  (set `self.SpawnTransform` (`self.GetTransform` (`|GetArrayItem` _outactors)))
  (`self.SpawnShape`)
  (add `self.GameOver` (`|CreateDelegate` :!event `OnGameOver`)))

(event `SpawnShape`
  (bind _shapes (`self.Shapes`))
  (`|SpawnActorFromClass` (`|GetArrayItem` _shapes (`KismetMathLibrary.RandomInteger` (- (`KismetArrayLibrary.Array_Length` _shapes) 1))) (`self.SpawnTransform`) "Undefined" "OverrideRootScale" null null))

(event `OnGameOver`)

(fn `UserConstructionScript`)