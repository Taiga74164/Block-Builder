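; BP_Block is a tinted physics block that can be grabbed, released and registered with a Tower.
; Grab disables physics and attaches it to the handle; Release detaches it, restores physics with a slight downward velocity to prevent throwing, then calls AddBlock on any valid Tower.
; A DoOnce limits the hit sound to one play until the next Grab resets it.
; Tick tracks speed and movement, and construction applies BlockColor through a dynamic material.
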(event `self.ReceiveBeginPlay`
  (set `self.Speed` 1000.0)
  (set `self.isMoving` true))

(event `self.ReceiveTick`
  (params (DeltaSeconds :type "Float (single-precision)"))
  ;[1 1 1] Tick
  (set `self.Speed` (`KismetMathLibrary.VSize` (`self.GetVelocity`)))
  (set `self.isMoving` (select `bool` (> (`self.Speed`) 0.0) :`false` false :`true` true)))

(event `/Game/Blueprints/BPI_Grab.Grab`
  (params (GrabHandle :type "SceneComponent Object Reference"))
  ;[0 0.1776 1 1 50] Grab
  ;;[1 1 1] Disable Physics
  (`PrimitiveComponent.SetSimulatePhysics` (`self.StaticMesh`) false)
  ;;[1 1 1] Attach to grab point on other actor
  (`self.K2_AttachToComponent` GrabHandle "None" "KeepWorld" "KeepWorld" "KeepWorld" false)
  (`self.Reset Sound Cue`))

(event `/Game/Blueprints/BPI_Grab.Release`
  (bind _tower (`self.Tower`))
  ;[0 1 0.25 1 50] Release
  ;;[1 1 1] Detach from grab handle
  (`self.K2_DetachFromActor` "KeepRelative")
  ;;[1 1 1] turn physics back on
  (`PrimitiveComponent.SetSimulatePhysics` (`self.StaticMesh`) true)
  ;;[1 1 1] prevent player from throwing object up into the air
  (`PrimitiveComponent.SetPhysicsLinearVelocity` (`self.StaticMesh`) (0.0 0.0 -1.0) false "None")
  (`/Engine/EditorBlueprintResources/StandardMacros.IsValid` _tower
    (:`Is Valid`
      (`/Game/Blueprints/BP_Tower.AddBlock` _tower self))))

(event `self.StaticMesh.OnComponentHit`
  (params (HitComponent :type "PrimitiveComponent Object Reference") (OtherActor :type "Actor Object Reference") (OtherComp :type "PrimitiveComponent Object Reference") (NormalImpulse :type "Vector Structure") (Hit :type "HitResult Structure (by ref)"))
  (`/Engine/EditorBlueprintResources/StandardMacros.DoOnce` false :!label _label
    (:`Completed`
      (`GameplayStatics.PlaySoundAtLocation` "/Game/Audio/Impacts_Soft_-_Short__Crack.Impacts_Soft_-_Short__Crack" (`SceneComponent.K2_GetComponentLocation` (`self.StaticMesh`)) (struct) 1.0 1.0 0.0 null null null null))))

(event `Reset Sound Cue`
  (goto _label :!via `Reset`))

(fn `UserConstructionScript`
  (bind _returnvalue (`PrimitiveComponent.CreateDynamicMaterialInstance` (`self.StaticMesh`) 0 "/Game/Materials/M_Block.M_Block" "None"))
  (set `self.DynamicMaterial` _returnvalue)
  (`MaterialInstanceDynamic.SetVectorParameterValue` (`self.DynamicMaterial`) "Tint" (`self.BlockColor`)))