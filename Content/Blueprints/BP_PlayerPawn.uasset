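; Player pawn that lets the mouse cursor grab, move, push/pull and rotate shapes in the world.
; Select line-traces under the cursor, passes GrabHandle to the hit actor via a grab message, then keeps the handle at GrabDistance along the cursor ray.
; A higher-priority holding input context is active during a grab, with rotation axes derived from the camera.
; It binds to the single-player game mode's game-over event, but OnGameOver is empty.
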(event `self.ReceiveBeginPlay`
  (bind _returnvalue (`GameplayStatics.GetPlayerController` 0))
  ;[1 0.0458 0 1 50] Begin Play
  (set `PlayerController.bShowMouseCursor` true _returnvalue)
  ;;[1 1 1] Enable grabbing objects
  (`EnhancedInputSubsystemInterface.AddMappingContext` (pcsubsystem `EnhancedInputLocalPlayerSubsystem` _returnvalue) "/Game/Input/IMC_SelectingShape.IMC_SelectingShape" 0 (struct))
  (bind _asbp_single_player_game_mode (cast `/Game/Blueprints/GameModes/BP_SinglePlayer_GameMode` (`GameplayStatics.GetGameMode`)))
  (add `/Game/Blueprints/GameModes/BP_SinglePlayer_GameMode.GameOver` _asbp_single_player_game_mode (`|CreateDelegate` :!event `OnGameOver`)))

(event `OnGameOver`)

(event `EnhancedInput|/Game/Input/IA_Select`
  (params (ActionValue :type Boolean) (ElapsedSeconds :type "Float (double-precision)") (TriggeredSeconds :type "Float (double-precision)") (InputAction :type "InputAction Object Reference" :default "/Game/Input/IA_Select.IA_Select"))
  (bind (_worldlocation _worlddirection) (`PlayerController.DeprojectMousePositionToWorld` (`GameplayStatics.GetPlayerController` 0)))
  (bind (_worldlocation_2 _worlddirection_2) (`PlayerController.DeprojectMousePositionToWorld` (`GameplayStatics.GetPlayerController` 0)))
  (bind (_worldlocation_3 _worlddirection_3) (`PlayerController.DeprojectMousePositionToWorld` (`GameplayStatics.GetPlayerController` 0)))
  (bind _returnvalue (+ _worldlocation_3 (* _worlddirection_3 (`self.GrabDistance`))))
  ;[0 0.25 1 1 50] Select
  (:`Triggered`
    ;;[1 1 1 1 30] Select Triggered/Hold on to object
    (`KismetSystemLibrary.DrawDebugSphere` _returnvalue 10.0)
    (`SceneComponent.K2_SetWorldLocation` (`self.GrabHandle`) _returnvalue false false))
  (:`Started`
    ;;[1 1 1 1 30] Select Started/grab object
    ;;;[1 1 1] Object
    (bind (_outhit _returnvalue_2) (`KismetSystemLibrary.LineTraceSingle` :`Start` _worldlocation_2 :`End` (+ _worldlocation_2 (* _worlddirection_2 100000.0)) :`TraceChannel` "TraceTypeQuery1" :`DrawDebugType` "ForDuration"))
    (set `self.Grab Hit Result` _outhit)
    (if _returnvalue_2
      (set `self.HeldActor` (`.HitActor` (`GameplayStatics.BreakHitResult` (`self.Grab Hit Result`))))
      (set `self.GrabDistance` (`.Distance` (`GameplayStatics.BreakHitResult` (`self.Grab Hit Result`))))
      ;;;[1 1 1] Update Grab Handle Position
      (`SceneComponent.K2_SetWorldLocation` (`self.GrabHandle`) (+ _worldlocation (* _worlddirection (`self.GrabDistance`))) false false)
      ;;;[1 1 1] Call Grab Interface
      (message `/Game/Blueprints/BPI_Grab.Grab` (`self.HeldActor`) (`self.GrabHandle`))
      ;;[1 1 1] enable item moving controls
      (`EnhancedInputSubsystemInterface.AddMappingContext` (pcsubsystem `EnhancedInputLocalPlayerSubsystem` (`GameplayStatics.GetPlayerController` 0)) "/Game/Input/IMC_HoldingShape.IMC_HoldingShape" 1 (struct))))
  (:`Completed`
    ;;[1 1 1 1 30] Select Ended/Let go of Object
    (message `/Game/Blueprints/BPI_Grab.Release` (`self.HeldActor`))
    (set `self.HeldActor` null)
    ;;[1 1 1] disable item moving controls
    (`EnhancedInputSubsystemInterface.RemoveMappingContext` (pcsubsystem `EnhancedInputLocalPlayerSubsystem` (`GameplayStatics.GetPlayerController` 0)) "/Game/Input/IMC_HoldingShape.IMC_HoldingShape" (struct))))

(event `EnhancedInput|/Game/Input/IA_Push`
  (params (ActionValue :type "Float (double-precision)") (ElapsedSeconds :type "Float (double-precision)") (TriggeredSeconds :type "Float (double-precision)") (InputAction :type "InputAction Object Reference" :default "/Game/Input/IA_Push.IA_Push"))
  ;[1 0 0.8727 1 50] Push/Pull Held Item
  (:`Triggered`
    ;;[1 1 1] Grab distance updates grab handle position as long as we are holding an object. This is done in the triggered section of IA_Select
    (set `self.GrabDistance` (+ (* (* ActionValue (`self.GrabMoveSpeed`)) (`GameplayStatics.GetWorldDeltaSeconds`)) (`self.GrabDistance`)))))

(event `EnhancedInput|/Game/Input/IA_Rotate`
  (params (ActionValue :type "Vector2D Structure") (ElapsedSeconds :type "Float (double-precision)") (TriggeredSeconds :type "Float (double-precision)") (InputAction :type "InputAction Object Reference" :default "/Game/Input/IA_Rotate.IA_Rotate"))
  (bind (_x _y) (`KismetMathLibrary.BreakVector2D` ActionValue))
  ;[0.1684 1 0 1 50] Rotate Held Item
  (:`Triggered`
    (`|ExecutionSequence`
      (:`then_0`
        ;;[1 1 1] roll object around camera forward vector
        (`self.K2_AddActorLocalRotation` (`self.HeldActor`) (`KismetMathLibrary.RotatorFromAxisAndAngle` (`KismetMathLibrary.Normal` (- (`SceneComponent.K2_GetComponentLocation` (`self.Camera`)) (`self.K2_GetActorLocation` (`self.HeldActor`)))) (* _x (* (`self.GrabRotateRate`) (`GameplayStatics.GetWorldDeltaSeconds`)))) false false))
      (:`then_1`
        ;;[1 1 1] rotate object around camera right vector
        (`self.K2_AddActorLocalRotation` (`self.HeldActor`) (`KismetMathLibrary.RotatorFromAxisAndAngle` (`SceneComponent.GetRightVector` (`self.Camera`)) (* _y (* (`self.GrabRotateRate`) (`GameplayStatics.GetWorldDeltaSeconds`)))) false false)))))

(fn `UserConstructionScript`)