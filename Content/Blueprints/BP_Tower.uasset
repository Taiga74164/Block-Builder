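; BP_Tower manages the block stack in a single-player stacking game, tracking its state from placing a block through release, stable and game over.
; Its volume hands a tower reference to overlapping blocks, and AddBlock registers them, marking them released after a brief delay.
; Tick then waits until no block is moving before asking the game mode to spawn the next shape.
; Any block except the first hitting the base triggers game over.
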(event `self.ReceiveBeginPlay`
  ;[1 1 1] Begin Play
  (set `self.TowerState` "NewEnumerator2")
  (bind _asbp_single_player_game_mode (cast `/Game/Blueprints/GameModes/BP_SinglePlayer_GameMode` (`GameplayStatics.GetGameMode`)))
  (bind _output_get (set `self.GameMode` _asbp_single_player_game_mode))
  (add `/Game/Blueprints/GameModes/BP_SinglePlayer_GameMode.GameOver` _output_get (`|CreateDelegate` :!event `OnGameOver`)))

(event `OnGameOver`
  (set `self.TowerState` "NewEnumerator3")
  (`KismetArrayLibrary.Array_Clear` (`self.blocks`)))

(event `self.ReceiveTick`
  (params (DeltaSeconds :type "Float (single-precision)"))
  ;[1 1 1] Tick
  (`|ExecutionSequence`
    (:`then_0`
      ;;[1 1 1] check stability
      (switch `/Game/Blueprints/ETowerState` (`self.TowerState`)
        (:`NewEnumerator1`
          (for _array_element (`self.blocks`)
            (set `self.IsStable` true)
            (`/Engine/EditorBlueprintResources/StandardMacros.IsValid` _array_element
              (:`Is Valid`
                (if (`/Game/Blueprints/Blocks/BP_Block.isMoving` _array_element)
                  (set `self.IsStable` false)
                  (break)))))
          (if (`self.IsStable`)
            (set `self.TowerState` "NewEnumerator2")
            (`/Game/Blueprints/GameModes/BP_SinglePlayer_GameMode.SpawnShape` (cast `/Game/Blueprints/GameModes/BP_SinglePlayer_GameMode` (`GameplayStatics.GetGameMode`) :!pure true))))))
    (:`then_1`
      (`KismetSystemLibrary.PrintString` (`KismetStringLibrary.Concat_StrStr` "Tower State: " (`|GetEnumeratorNameAsString` (`self.TowerState`))) true true (struct :`G` 0.66 :`B` 1.0 :`A` 1.0) 2.0 "1"))))

(event `self.Base.OnComponentHit`
  (params (HitComponent :type "PrimitiveComponent Object Reference") (OtherActor :type "Actor Object Reference") (OtherComp :type "PrimitiveComponent Object Reference") (NormalImpulse :type "Vector Structure") (Hit :type "HitResult Structure (by ref)"))
  ;[1 1 1] base hit event
  (if (== (`KismetArrayLibrary.Array_Length` (`self.blocks`)) 1)
    (set `self.FirstBlock` (cast `/Game/Blueprints/Blocks/BP_Block` OtherActor :!pure true))
    (elif (!= (`self.FirstBlock`) OtherActor)
      (`/Game/Blueprints/GameModes/BP_SinglePlayer_GameMode.GameOver` (`self.GameMode`)))))

(event `AddBlock`
  (params (Block :type "/Game/Blueprints/Blocks/BP_Block Object Reference"))
  ;[1 1 1] add block to tower
  (`KismetArrayLibrary.Array_Add` (`self.blocks`) Block)
  (`KismetSystemLibrary.Delay` 0.01)
  (set `self.TowerState` "NewEnumerator1"))

(event `self.tower_volume.OnComponentBeginOverlap`
  (params (OverlappedComponent :type "PrimitiveComponent Object Reference") (OtherActor :type "Actor Object Reference") (OtherComp :type "PrimitiveComponent Object Reference") (OtherBodyIndex :type Integer) (bFromSweep :type Boolean) (SweepResult :type "HitResult Structure (by ref)"))
  (bind (_asbp_block _bsuccess) (cast `/Game/Blueprints/Blocks/BP_Block` OtherActor :!pure true))
  ;[1 1 1] On tower volume overlap
  ;;[1 1 1] pass reference to self to block object
  (if _bsuccess
    (set `/Game/Blueprints/Blocks/BP_Block.Tower` self _asbp_block)
    (set `self.TowerState` "NewEnumerator0")))

(fn `UserConstructionScript`)